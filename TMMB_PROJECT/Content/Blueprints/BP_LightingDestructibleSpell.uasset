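; BP_LightingDestructibleSpell is a destructible spell actor that sparks when it breaks and applies force to the player on contact.
; On fracture, it spawns an enlarged spark emitter at the hit point, then destroys the emitter and itself after a short delay.
; On hit, it filters for the Player tag and Elementalist class, then pushes that capsule with a scaled, inverted normal impulse.
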(event `self.DestructibleComponent.OnComponentFracture`
  (params (HitPoint :type "Vector Structure (by ref)") (HitDirection :type "Vector Structure (by ref)"))
  (bind _returnvalue (`GameplayStatics.SpawnEmitterAtLocation` "/Game/StarterContent/Particles/P_Sparks.P_Sparks" HitPoint (struct) (15.0 15.0 15.0) false))
  (`KismetSystemLibrary.Delay` 5.0)
  (`ActorComponent.K2_DestroyComponent` _returnvalue)
  (`self.K2_DestroyActor`))

(event `self.DestructibleComponent.OnComponentHit`
  (params (HitComponent :type "PrimitiveComponent Object Reference") (OtherActor :type "Actor Object Reference") (OtherComp :type "PrimitiveComponent Object Reference") (NormalImpulse :type "Vector Structure") (Hit :type "HitResult Structure (by ref)"))
  (if (`self.ActorHasTag` OtherActor "Player")
    (bind _aselementalist (cast `Elementalist` OtherActor))
    (`PrimitiveComponent.AddForce` (`BaseCaster.CapsuleComponent` _aselementalist) (* NormalImpulse -1000.0) "None" false)))

(fn `UserConstructionScript`)