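; Game manager that periodically spawns mana potions at random TargetPoints in the level.
; BeginPlay caches all TargetPoint actors, and a Delay on Tick throttles calls to SpawnPotion.
; SpawnPotion randomly picks a red, green or blue potion class and builds its transform from randomly indexed points, replacing Z with SpawnHeight.
; Debug prints mark each spawn call.
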(event `self.ReceiveBeginPlay`
  (bind _outactors (`GameplayStatics.GetAllActorsOfClass` "/Script/Engine.TargetPoint"))
  (set `self.FoundSpawnPoints` _outactors))

(event `self.ReceiveTick`
  (params (DeltaSeconds :type "Float (single-precision)"))
  (`KismetSystemLibrary.Delay` 12.0)
  (`KismetSystemLibrary.PrintString` "callspawnevent")
  (`self.SpawnPotion`))

(event `SpawnPotion`
  (bind _spawnheight (`self.spawnHeight`))
  (bind _foundspawnpoints (`self.FoundSpawnPoints`))
  (bind _returnvalue (`self.GetTransform` (`|GetArrayItem` _foundspawnpoints (`KismetMathLibrary.RandomInteger` (`KismetArrayLibrary.Array_Length` _foundspawnpoints)))))
  (switch `int` (`KismetMathLibrary.RandomInteger` 3)
    (:`Default`
      (`|SpawnActorFromClass` "/Game/Blueprints/ManaPotions/BP_ManaPotionRed.BP_ManaPotionRed_C" (`KismetMathLibrary.MakeTransform` (`KismetMathLibrary.MakeVector` (.x (.location _returnvalue)) (.y (.location _returnvalue)) _spawnheight) (.rotation _returnvalue) (.scale _returnvalue)) "Undefined" "OverrideRootScale" null null :!label _label))
    (:`0`
      (goto _label))
    (:`1`
      (`|SpawnActorFromClass` "/Game/Blueprints/ManaPotions/BP_ManaPotionGreen.BP_ManaPotionGreen_C" (`KismetMathLibrary.MakeTransform` (`KismetMathLibrary.MakeVector` (.x (.location _returnvalue)) (.y (.location _returnvalue)) _spawnheight) (.rotation _returnvalue) (.scale _returnvalue)) "Undefined" "OverrideRootScale" null null))
    (:`2`
      (`|SpawnActorFromClass` "/Game/Blueprints/ManaPotions/BP_ManaPotionBlue.BP_ManaPotionBlue_C" (`KismetMathLibrary.MakeTransform` (`KismetMathLibrary.MakeVector` (.x (.location _returnvalue)) (.y (.location _returnvalue)) _spawnheight) (.rotation _returnvalue) (.scale _returnvalue)) "Undefined" "OverrideRootScale" null null)))
  (`KismetSystemLibrary.PrintString` "FinsihedCallingEvent"))

(fn `UserConstructionScript`)