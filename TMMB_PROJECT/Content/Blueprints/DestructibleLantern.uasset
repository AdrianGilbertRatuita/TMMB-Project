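; Destructible lantern actor that cleans up its debris after it breaks.
; When the Destructible component fractures, a delay leaves the pieces in place for a few seconds before setting the Fractured flag.
; Tick then shrinks the actor's scale linearly with delta time, and the actor destroys itself about a second later, as a unit scale reaches zero.
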(event `self.ReceiveTick`
  (params (DeltaSeconds :type "Float (single-precision)"))
  (if (`self.Fractured`)
    (`self.SetActorScale3D` (- (`self.GetActorScale3D`) (* (1.0 1.0 1.0) DeltaSeconds)))))

(event `self.Destructible.OnComponentFracture`
  (params (HitPoint :type "Vector Structure (by ref)") (HitDirection :type "Vector Structure (by ref)"))
  (`KismetSystemLibrary.Delay` 5.0)
  (set `self.Fractured` true)
  (`KismetSystemLibrary.Delay` 1.0)
  (`self.K2_DestroyActor`))

(fn `UserConstructionScript`)